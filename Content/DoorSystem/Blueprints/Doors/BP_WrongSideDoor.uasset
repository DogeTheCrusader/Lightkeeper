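; Double door that opens only when interacted with from the correct side.
; Two overlap triggers set a side state that the interaction event reads.
; From the right side, timelines rotate both leaves open, with the left started from the right's update, and the wrong-side trigger's collision is disabled.
; From the wrong side, it shows a notification widget, guarded against duplicates until a short delay clears the reference.
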(event OnComponentBeginOverlap(RightSideTrigger)
  (params (OverlappedComponent :type Primitive%20Component%20Object%20Reference) (OtherActor :type Actor%20Object%20Reference) (OtherComp :type Primitive%20Component%20Object%20Reference) (OtherBodyIndex :type Integer) (bFromSweep :type Boolean) (SweepResult :type Hit%20Result%20Structure%20%28by%20ref%29))
  (Variables|Default|SetDoorStates "NewEnumerator1"))

(event OnComponentEndOverlap(RightSideTrigger)
  (params (OverlappedComponent :type Primitive%20Component%20Object%20Reference) (OtherActor :type Actor%20Object%20Reference) (OtherComp :type Primitive%20Component%20Object%20Reference) (OtherBodyIndex :type Integer))
  (Variables|Default|SetDoorStates "NewEnumerator0"))

(event OnComponentBeginOverlap(WrongSideTrigger)
  (params (OverlappedComponent :type Primitive%20Component%20Object%20Reference) (OtherActor :type Actor%20Object%20Reference) (OtherComp :type Primitive%20Component%20Object%20Reference) (OtherBodyIndex :type Integer) (bFromSweep :type Boolean) (SweepResult :type Hit%20Result%20Structure%20%28by%20ref%29))
  (Variables|Default|SetDoorStates "NewEnumerator2"))

(event OnComponentEndOverlap(WrongSideTrigger)
  (params (OverlappedComponent :type Primitive%20Component%20Object%20Reference) (OtherActor :type Actor%20Object%20Reference) (OtherComp :type Primitive%20Component%20Object%20Reference) (OtherBodyIndex :type Integer))
  (Variables|Default|SetDoorStates "NewEnumerator0"))

(event EventOnInteraction
  (params (Player%20Ref :type BP%20Third%20Person%20Character%20Object%20Reference))
  (switch Utilities|FlowControl|Switch|SwitchonE_WrongDoorSideStates (Variables|Default|GetDoorStates)
    (:NewEnumerator1
      (bind _door_timer (Timeline|RightDoor Play)
        (:Update
          (Transformation|SetRelativeRotation (Variables|Default|GetRightSide) (Math|Rotator|MakeRotator 0.0 0.0 (Math|Float|Lerp -1.8e+02 -6e+01 _door_timer)) false false)
          (bind _door_timer_2 (Timeline|LeftDoor Play)
            (:Update
              (Transformation|SetRelativeRotation (Variables|Default|GetLeftSide) (Math|Rotator|MakeRotator 0.0 0.0 (Math|Float|Lerp 0.0 -1.1e+02 _door_timer_2)) false false)
              (Collision|SetCollisionEnabled (Variables|Default|GetWrongSideTrigger) "NoCollision"))))))
    (:NewEnumerator2
      (Utilities|IsValid (Variables|Default|GetNotificationWidget)
        (:Is%20Not%20Valid
          (bind _returnvalue (UserInterface|CreateWidget "/Game/DoorSystem/Player/Widgets/WBP_WrongSide.WBP_WrongSide_C" 0 "Can't Open From This Side!"))
          (bind _output_get (Variables|Default|SetNotificationWidget _returnvalue))
          (UserInterface|Viewport|AddtoViewport _output_get 0)
          (Utilities|FlowControl|Delay 1.5)
          (Variables|Default|SetNotificationWidget 0))))))

(fn ConstructionScript)