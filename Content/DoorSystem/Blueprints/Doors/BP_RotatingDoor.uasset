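; BP_RotatingDoor is a rotating door that spins while its trigger box is overlapped.
; Box begin and end overlap events set and clear an InBox flag, with no filter on the overlapping actor or count of overlaps.
; While the flag is set, Tick adds local yaw to the Cylinder, scaled by RotationSpeed and delta time for frame-rate independent motion.
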(event OnComponentBeginOverlap(Box)
  (params (OverlappedComponent :type Primitive%20Component%20Object%20Reference) (OtherActor :type Actor%20Object%20Reference) (OtherComp :type Primitive%20Component%20Object%20Reference) (OtherBodyIndex :type Integer) (bFromSweep :type Boolean) (SweepResult :type Hit%20Result%20Structure%20%28by%20ref%29))
  (Variables|Default|SetInBox true))

(event OnComponentEndOverlap(Box)
  (params (OverlappedComponent :type Primitive%20Component%20Object%20Reference) (OtherActor :type Actor%20Object%20Reference) (OtherComp :type Primitive%20Component%20Object%20Reference) (OtherBodyIndex :type Integer))
  (Variables|Default|SetInBox false))

(event EventTick
  (params (DeltaSeconds :type Float%20%28single-precision%29))
  (if (Variables|Default|GetInBox)
    (Transformation|AddLocalRotation (Variables|Default|GetCylinder) (Math|Rotator|MakeRotator 0.0 0.0 (* DeltaSeconds (Variables|Default|GetRotationSpeed))) false false)))

(fn ConstructionScript)