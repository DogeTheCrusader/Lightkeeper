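; Base physics door for Lightkeeper that the player grabs and swings, starting either latched or ajar.
; Grabbing nudges a latched door free and enables physics; move input adds yaw angular velocity, signed by the player's side and scaled by movement resistance.
; Tick auto-latches a released door within a few degrees of closed via a timeline snap, while locked interaction plays a rattle.
; SlamObject is empty; its slam logic is disconnected.
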(event EventBeginPlay
  ;[0.15 0.15 0.15 0.5] initialize
  (Variables|Default|SetClosedYawPosition (.Yaw (Math|Rotator|BreakRotator (Transformation|GetActorRotation))))
  (if (> (Variables|Default|GetInitialOpenAngle) 5.0)
    (Transformation|SetRelativeRotation (Variables|Default|GetDoor) (Math|Rotator|MakeRotator 0.0 0.0 (+ (Variables|Default|GetClosedYawPosition) (Variables|Default|GetInitialOpenAngle))) false false)
    (Physics|SetSimulatePhysics (Variables|Default|GetDoor) true)
    (Variables|Default|SetbIsLatched false)
    (else
      (Physics|SetSimulatePhysics (Variables|Default|GetDoor) false)
      (Variables|Default|SetbIsLatched true))))

(event EventMoveObject
  (params (AxisDelta :type Float%20%28single-precision%29))
  (bind _self self)
  ;[0.15 0.15 0.15 0.5] move door
  (bind _output_get (Variables|Default|SetisFacing (>= (Math|Vector|DotProduct (Math|Vector|Normalize (- (Transformation|GetActorLocation _self) (Transformation|GetActorLocation (Game|GetPlayerCharacter 0)))) (Transformation|GetActorForwardVector _self)) 0.0)))
  (bind _output_get_2 (Variables|Default|SetDirFacing (select _output_get 1.0 -1.0)))
  (Class|PrimitiveComponent|SetPhysicsAngularVelocityinDegrees (Variables|Default|GetDoor) (Math|Vector|MakeVector 0.0 0.0 (* (* (Variables|Default|GetBaseInteractionPower) (* AxisDelta _output_get_2)) (Class|BaseInteractable|CalculateMovementResistance (Variables|Default|GetDoor)))) true "None"))

(event EventSlamObject
  (params (PushDirection :type Vector :default "0, 0, 0") (PushForce :type Float%20%28single-precision%29))
  ;[0.15 0.15 0.15 0.5] slam
)

(event EventOnLockedInteraction
  (params (InstigatorActor :type Actor%20Object%20Reference))
  ;[0.15 0.15 0.15 0.5] locked rattle
  (Development|PrintString (Utilities|String|ToString(Float) (Variables|Default|GetClosedYawPosition)))
  (Development|PrintString (Utilities|String|ToString(Rotator) (Variables|/Script/Engine.SceneComponent|GetRelativeRotation (Variables|Default|GetDoor))))
  (|CallParentFunction InstigatorActor)
  (bind _yawoffset (Timeline|TL_DoorRattle PlayFromStart)
    (:Update
      (Transformation|SetRelativeRotation (Variables|Default|GetDoor) (Math|Rotator|MakeRotator 0.0 0.0 (+ _yawoffset (Variables|Default|GetClosedYawPosition))) false false))
    (:Finished
      (Transformation|SetRelativeRotation (Variables|Default|GetDoor) (Math|Rotator|MakeRotator 0.0 0.0 (Variables|Default|GetClosedYawPosition)) false false))))

(event EventGrabObject
  (params (Grabber :type Actor%20Object%20Reference))
  ;[0.15 0.15 0.15 0.5] grab door
  (Audio|Components|Audio|Stop (Variables|Default|GetTL_SmoothLatch))
  (Variables|Default|SetbIsAutoLatching false)
  (Class|PrimitiveComponent|SetPhysicsAngularVelocityinDegrees (Variables|Default|GetDoor) "0, 0, 0" false "None")
  (Development|PrintString "klik")
  (Development|PrintString (Utilities|String|ToString(Float) (Variables|Default|GetClosedYawPosition)))
  (Development|PrintString (Utilities|String|ToString(Rotator) (Variables|/Script/Engine.SceneComponent|GetRelativeRotation (Variables|Default|GetDoor))))
  (if (Variables|Default|GetbIsLatched)
    (bind _output_get (Variables|Default|SetStartAngle (.Yaw (Math|Rotator|BreakRotator (Variables|/Script/Engine.SceneComponent|GetRelativeRotation (Variables|Default|GetDoor))))))
    (bind _newtrack_0 (Timeline|TL_Nudge PlayFromStart)
      (:Update
        (Transformation|SetRelativeRotation (Variables|Default|GetDoor) (Math|Rotator|MakeRotator 0.0 0.0 (+ _output_get _newtrack_0)) false false))
      (:Finished
        (Physics|SetSimulatePhysics (Variables|Default|GetDoor) true)))
    (Variables|Default|SetbIsLatched false))
  (|CallParentFunction Grabber)
  (Physics|SetSimulatePhysics (Variables|Default|GetDoor) true)
  (Class|PrimitiveComponent|SetPhysicsAngularVelocityinDegrees (Variables|Default|GetDoor) "0, 0, 0" false "None"))

(event EventReleaseObject
  ;[0.15 0.15 0.15 0.5] release door
  (|CallParentFunction)
  (Class|PrimitiveComponent|SetPhysicsAngularVelocityinDegrees (Variables|Default|GetDoor) "0, 0, 0" false "None"))

(event EventTick
  (params (DeltaSeconds :type Float%20%28single-precision%29))
  (bind _door (Variables|Default|GetDoor))
  (bind _door_2 (Variables|Default|GetDoor))
  (bind _closedyawposition (Variables|Default|GetClosedYawPosition))
  (bind _relativerotation (Variables|/Script/Engine.SceneComponent|GetRelativeRotation _door_2))
  (bind _yaw (Math|Rotator|BreakRotator _relativerotation))
  (bind _returnvalue (- _yaw _closedyawposition))
  (bind _returnvalue_2 (Math|Rotator|NormalizeAxis _returnvalue))
  (bind _returnvalue_3 (Math|Float|Absolute(Float) _returnvalue_2))
  (bind _returnvalue_4 (< _returnvalue_3 5.0))
  ;[0.15 0.15 0.15 0.5] auto latch
  (Variables|Default|SetbEnableAutoLatch _returnvalue_4)
  (if (Variables|Default|GetbEnableAutoLatch)
    (if (not (Variables|Default|GetbIsHeld))
      (if (not (Variables|Default|GetbIsLatched))
        (if (Physics|IsSimulatingPhysics (Variables|Default|GetDoor) "None")
          (if _returnvalue_4
            (if (not (Variables|Default|GetbIsAutoLatching))
              (Variables|Default|SetbIsAutoLatching true)
              (Class|PrimitiveComponent|SetPhysicsAngularVelocityinDegrees (Variables|Default|GetDoor) "0, 0, 0" false "None")
              (Physics|SetSimulatePhysics _door false)
              (bind _output_get (Variables|Default|SetStartSnap (.Yaw (Math|Rotator|BreakRotator (Variables|/Script/Engine.SceneComponent|GetRelativeRotation _door)))))
              (bind _newtrack_0 (Timeline|TL_SmoothLatch PlayFromStart)
                (:Update
                  (Transformation|SetRelativeRotation (Variables|Default|GetDoor) (Math|Rotator|MakeRotator 0.0 0.0 (Math|Float|Lerp _output_get (Variables|Default|GetClosedYawPosition) _newtrack_0)) false false))
                (:Finished
                  (Transformation|SetRelativeRotation (Variables|Default|GetDoor) (Math|Rotator|MakeRotator 0.0 0.0 (Variables|Default|GetClosedYawPosition)) false false)
                  (Variables|Default|SetbIsLatched true)
                  (Variables|Default|SetbIsAutoLatching false)
                  (Class|PrimitiveComponent|SetPhysicsAngularVelocityinDegrees (Variables|Default|GetDoor) "0, 0, 0" false "None"))))))))))

(fn ConstructionScript
  (|CallParentFunction))