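; BP_BaseBolt is a base sliding bolt interactable that locks and unlocks its parent actor when grabbed.
; A FlipFlop on GrabObject alternates between sliding the bolt mesh aside to unlock and back to lock.
; It pushes lock state to the parent actor through message calls, and only closes if that parent reports it is latched.
; The FlipFlop still advances when that check fails, so the next grab runs the unlock branch again.
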(event EventGrabObject
  (params (Grabber :type Actor%20Object%20Reference))
  (|CallParentFunction Grabber)
  (Utilities|FlowControl|FlipFlop
    (:A
      (Components|MoveComponentTo (Variables|Default|GetBoltMesh) "0.000000,15.000000,0.000000" "0, 0, 0" false false 0.15 false)
      (Variables|Default|SetbIsLatched false)
      (Class|PhysicalInteract|SetLocked false)
      (Class|PhysicalInteract|SetLocked(Message) (Actor|GetParentActor) false))
    (:B
      (bind _returnvalue (Class|PhysicalInteract|IsLatched(Message) (Actor|GetParentActor)))
      (if _returnvalue
        (Components|MoveComponentTo (Variables|Default|GetBoltMesh) "0, 0, 0" "0, 0, 0" false false 0.15 false)
        (Variables|Default|SetbIsLatched true)
        (Class|PhysicalInteract|SetLocked true)
        (Class|PhysicalInteract|SetLocked(Message) (Actor|GetParentActor) true)))))

(fn ConstructionScript
  (|CallParentFunction))