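; Base class for sliding interactables such as doors, which the player grabs and pushes along the mesh's forward, right or up axis.
; Move input, scaled by interaction power and movement resistance, drives a clamped slide distance that Tick smoothly interpolates into the non-physics mesh's relative location.
; Forward sliders derive their travel limit from mesh bounds.
; Grabbing unlatches it; releasing or slamming while held near closed latches it.
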(event EventBeginPlay
  (bind _mesh (Variables|Default|GetMesh))
  (bind _mesh_2 (Variables|Default|GetMesh))
  (bind (_min _max) (Components|StaticMesh|GetLocalBounds _mesh_2))
  ;[0.15 0.15 0.15 0.5] initialize
  (Physics|SetSimulatePhysics _mesh false)
  (Variables|Default|SetInitialRestLocation (Variables|/Script/Engine.SceneComponent|GetRelativeLocation _mesh))
  (if (Utilities|Enum|Equal(Enum) (Variables|Default|GetSlideDirection) "NewEnumerator0")
    (Variables|Default|SetMaxOpenDist (* (.Y (Math|Vector|BreakVector (- _max _min))) 0.8)))
  (if (> (Variables|Default|GetInitialSlideOffset) 1.0)
    (Variables|Default|SetSlideDistance (Variables|Default|GetInitialSlideOffset))
    (Variables|Default|SetbIsLatched false)))

(event EventSlamObject
  (params (PushDirection :type Vector :default "0, 0, 0") (PushForce :type Float%20%28single-precision%29))
  (Class|PhysicalInteract|ReleaseObject))

(event EventTick
  (params (DeltaSeconds :type Float%20%28single-precision%29))
  ;[0.15 0.15 0.15 0.5] tick
  (|CallParentFunction DeltaSeconds)
  (Transformation|SetRelativeLocation (Variables|Default|GetMesh) (Math|Interpolation|VInterpTo (Variables|/Script/Engine.SceneComponent|GetRelativeLocation (Variables|Default|GetMesh)) (+ (* (Utilities|Select :Index (Variables|Default|GetSlideDirection) :NewEnumerator0 (Math|Vector|GetForwardVector (Variables|Default|GetMesh)) :NewEnumerator1 (Math|Vector|GetRightVector (Variables|Default|GetMesh)) :NewEnumerator5 (Math|Vector|GetUpVector (Variables|Default|GetMesh))) (Variables|Default|GetSlideDistance)) (Variables|Default|GetInitialRestLocation)) DeltaSeconds 8.0) false false))

(event EventGrabObject
  (params (Grabber :type Actor%20Object%20Reference))
  ;[0.15 0.15 0.15 0.5] grab door
  (Variables|Default|SetbIsLatched false)
  (|CallParentFunction Grabber)
  (Development|PrintString "klik"))

(event EventMoveObject
  (params (AxisDelta :type Float%20%28single-precision%29))
  ;[0.15 0.15 0.15 0.5] move door
  (Variables|Default|SetSlideDistance (Math|Float|Clamp(Float) (+ (* (* (* (Variables|Default|GetBaseInteractionPower) AxisDelta) (Class|BaseInteractable|CalculateMovementResistance (Variables|Default|GetMesh))) 0.05) (Variables|Default|GetSlideDistance)) 0.0 (Variables|Default|GetMaxOpenDist))))

(event EventReleaseObject
  ;[0.15 0.15 0.15 0.5] release door
  (Variables|Default|SetbIsLatched false)
  (if (and (<= (Variables|Default|GetSlideDistance) 1.0) (Variables|Default|GetbIsHeld))
    (Variables|Default|SetbIsLatched true))
  (|CallParentFunction))

(fn ConstructionScript)