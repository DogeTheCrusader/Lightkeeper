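; Base Blueprint for a grabbable crank that the player turns about its yaw axis between minimum and maximum rotation limits.
; While held, move input scaled by interaction power and movement resistance rotates the crank and sets a spin velocity.
; After release, Tick carries that spin on as inertia, easing it out by mechanical friction and stopping it at either limit.
; Slamming simply releases the crank.
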(event EventBeginPlay
  ;[0.15 0.15 0.15 0.5] initialize
  (Physics|SetSimulatePhysics (Variables|Default|GetCrank) false)
  (Variables|Default|SetCurrentRotation (Variables|Default|GetStartRotation))
  (Transformation|SetRelativeRotation (Variables|Default|GetCrank) (Math|Rotator|MakeRotator 0.0 0.0 (Variables|Default|GetStartRotation)) false false))

(event EventMoveObject
  (params (AxisDelta :type Float%20%28single-precision%29))
  (bind _baseinteractionpower (Variables|Default|GetBaseInteractionPower))
  (bind _crank (Variables|Default|GetCrank))
  (bind _returnvalue (Class|BaseInteractable|CalculateMovementResistance _crank))
  (bind _returnvalue_2 (* AxisDelta _baseinteractionpower))
  (bind _returnvalue_3 (* _returnvalue_2 _returnvalue))
  ;[0.15 0.15 0.15 0.5] move
  (Variables|Default|SetSpinVelocity (* _returnvalue_3 5.0))
  (Variables|Default|SetCurrentRotation (Math|Float|Clamp(Float) (+ (* _returnvalue_3 0.05) (Variables|Default|GetCurrentRotation)) (Variables|Default|GetMinRotation) (Variables|Default|GetMaxRotation)))
  (Transformation|AddLocalRotation (Variables|Default|GetCrank) (Math|Rotator|MakeRotator 0.0 0.0 (- (Math|Float|Clamp(Float) (+ (* _returnvalue_3 0.05) (Variables|Default|GetCurrentRotation)) (Variables|Default|GetMinRotation) (Variables|Default|GetMaxRotation)) (Variables|Default|GetCurrentRotation))) false false))

(event EventSlamObject
  (params (PushDirection :type Vector :default "0, 0, 0") (PushForce :type Float%20%28single-precision%29))
  (Class|PhysicalInteract|ReleaseObject))

(event EventGrabObject
  (params (Grabber :type Actor%20Object%20Reference))
  ;[0.15 0.15 0.15 0.5] grab door
  (|CallParentFunction Grabber))

(event EventReleaseObject
  ;[0.15 0.15 0.15 0.5] release
  (|CallParentFunction))

(event EventTick
  (params (DeltaSeconds :type Float%20%28single-precision%29))
  ;[0.15 0.15 0.15 0.5] poslizg
  (if (not (Variables|Default|GetbIsHeld))
    (if (> (Math|Float|Absolute(Float) (Variables|Default|GetSpinVelocity)) 0.01)
      (Variables|Default|SetCurrentRotation (Math|Float|Clamp(Float) (+ (* DeltaSeconds (Variables|Default|GetSpinVelocity)) (Variables|Default|GetCurrentRotation)) (Variables|Default|GetMinRotation) (Variables|Default|GetMaxRotation)))
      (Transformation|AddLocalRotation (Variables|Default|GetCrank) (Math|Rotator|MakeRotator 0.0 0.0 (- (Math|Float|Clamp(Float) (+ (* DeltaSeconds (Variables|Default|GetSpinVelocity)) (Variables|Default|GetCurrentRotation)) (Variables|Default|GetMinRotation) (Variables|Default|GetMaxRotation)) (Variables|Default|GetCurrentRotation))) false false)
      (Variables|Default|SetSpinVelocity (Math|Interpolation|FInterpTo (Variables|Default|GetSpinVelocity) 0.0 DeltaSeconds (Variables|Default|GetMechanicalFriction)))
      (if (or (== (Variables|Default|GetCurrentRotation) (Variables|Default|GetMinRotation)) (== (Variables|Default|GetCurrentRotation) (Variables|Default|GetMaxRotation)))
        (Variables|Default|SetSpinVelocity 0.0)))))

(fn ConstructionScript
  (|CallParentFunction))