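; Base physics prop that the player can grab, release and slam.
; Grab and release defer to the parent class, with grab also printing a debug message.
; Slamming a held prop applies an impulse to its mesh along the push direction, scaled by a slam force, then releases it.
; Older physics-handle hold and pawn-collision logic remains in the graph but is disconnected.
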(event EventGrabObject
  (params (Grabber :type Actor%20Object%20Reference))
  (Development|PrintString "podnoszenie")
  (|CallParentFunction Grabber))

(event EventTick
  (params (DeltaSeconds :type Float%20%28single-precision%29)))

(event EventReleaseObject
  (|CallParentFunction))

(event EventSlamObject
  (params (PushDirection :type Vector :default "0, 0, 0"))
  (Development|PrintString "rzut")
  (if (Variables|Default|GetbIsHeld)
    (Physics|AddImpulse (Variables|Default|GetPropMesh) (* PushDirection (Variables|Default|GetSlamForce)) "None" false)
    (Class|PhysicalInteract|ReleaseObject)))

(fn ConstructionScript
  (|CallParentFunction))