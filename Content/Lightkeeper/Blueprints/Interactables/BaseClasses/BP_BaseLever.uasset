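; Base grabbable lever that switches a mechanism on or off and drives the SafeLightComponent of a target light.
; Dragging rolls the lever within its limits, scaled by power and movement resistance, and crossing the midpoint sets TriggerSender's state, which is forwarded to the light.
; On release or slam, spin velocity projects which end to snap to, and Tick interpolates there without updating the trigger.
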(event OnMechanismStateChanged(TriggerSender)
  (params (bIsActivated :type Boolean))
  (bind _targetlight (Variables|Default|GetTargetLight))
  (bind _returnvalue (Actor|GetComponentbyClass _targetlight "/Script/Lightkeeper.SafeLightComponent"))
  (Utilities|IsValid _returnvalue
    (:Is%20Valid
      (Class|SafeLightComponent|SetLightActive _returnvalue bIsActivated))))

(event EventBeginPlay
  ;[0.15 0.15 0.15 0.5] initialize
  (Physics|SetSimulatePhysics (Variables|Default|GetLever) false)
  (bind _output_get (Variables|Default|SetCurrentRotation (Variables|Default|GetStartRotation)))
  (Transformation|SetRelativeRotation (Variables|Default|GetLever) (Math|Rotator|MakeRotator _output_get 0.0 0.0) false false))

(event EventMoveObject
  (params (AxisDelta :type Float%20%28single-precision%29))
  (bind _baseinteractionpower (Variables|Default|GetBaseInteractionPower))
  (bind _lever (Variables|Default|GetLever))
  (bind _returnvalue (Class|BaseInteractable|CalculateMovementResistance _lever))
  (bind _returnvalue_2 (* AxisDelta _baseinteractionpower))
  (bind _returnvalue_3 (* _returnvalue_2 _returnvalue))
  ;[0.15 0.15 0.15 0.5] move
  (Variables|Default|SetSpinVelocity (* _returnvalue_3 0.2))
  (bind _output_get (Variables|Default|SetCurrentRotation (Math|Float|Clamp(Float) (+ (* _returnvalue_3 0.05) (Variables|Default|GetCurrentRotation)) (Variables|Default|GetMinRotation) (Variables|Default|GetMaxRotation))))
  (Transformation|SetRelativeRotation (Variables|Default|GetLever) (Math|Rotator|MakeRotator _output_get 0.0 0.0) false false)
  (if (> (Variables|Default|GetCurrentRotation) (/ (+ (Variables|Default|GetMinRotation) (Variables|Default|GetMaxRotation)) 2.0))
    (Class|TriggerSenderComponent|SetMechanismActivated (Variables|Default|GetTriggerSender) true)
    (else
      (Class|TriggerSenderComponent|SetMechanismActivated (Variables|Default|GetTriggerSender) false))))

(event EventSlamObject
  (params (PushDirection :type Vector :default "0, 0, 0") (PushForce :type Float%20%28single-precision%29))
  (Class|PhysicalInteract|ReleaseObject))

(event EventGrabObject
  (params (Grabber :type Actor%20Object%20Reference))
  ;[0.15 0.15 0.15 0.5] grab
  (|CallParentFunction Grabber))

(event EventReleaseObject
  ;[0.15 0.15 0.15 0.5] release
  (|CallParentFunction)
  (if (> (+ (* (Variables|Default|GetSpinVelocity) 0.15) (Variables|Default|GetCurrentRotation)) (/ (+ (Variables|Default|GetMaxRotation) (Variables|Default|GetMinRotation)) 2.0))
    (Variables|Default|SetTargetSnapAngle (Variables|Default|GetMaxRotation))
    (else
      (Variables|Default|SetTargetSnapAngle (Variables|Default|GetMinRotation)))))

(event EventTick
  (params (DeltaSeconds :type Float%20%28single-precision%29))
  ;[0.15 0.15 0.15 0.5] poslizg
  (if (not (Variables|Default|GetbIsHeld))
    (if (> (Math|Float|Absolute(Float) (Variables|Default|GetSpinVelocity)) 0.01)
      (bind _output_get (Variables|Default|SetCurrentRotation (Math|Interpolation|FInterpTo (Variables|Default|GetCurrentRotation) (Variables|Default|GetTargetSnapAngle) DeltaSeconds 8.0)))
      (Transformation|SetRelativeRotation (Variables|Default|GetLever) (Math|Rotator|MakeRotator _output_get 0.0 0.0) false false))))

(fn ConstructionScript
  (|CallParentFunction))