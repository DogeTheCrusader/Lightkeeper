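; Base drawer interactable that the player grabs and slides open or shut along its local Y axis.
; Move input, scaled by interaction power and movement resistance, sets a slide distance clamped to 80% of the mesh's depth.
; Tick eases the non-simulated mesh toward that distance, and releasing or slamming a held drawer near closed latches it.
; The construction script still sets a physics constraint limit, and older physics and input-lock logic sits disconnected.
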(event EventBeginPlay
  (bind _drawermesh (Variables|Default|GetDrawerMesh))
  (bind _drawermesh_2 (Variables|Default|GetDrawerMesh))
  (bind (_min _max) (Components|StaticMesh|GetLocalBounds _drawermesh_2))
  ;[0.15 0.15 0.15 0.5] initialize
  (Physics|SetSimulatePhysics _drawermesh false)
  (Variables|Default|SetInitialRestLocation (Variables|/Script/Engine.SceneComponent|GetRelativeLocation _drawermesh))
  (Variables|Default|SetMaxOpenDist (* (.Y (Math|Vector|BreakVector (- _max _min))) 0.8)))

(event EventSlamObject
  (params (PushDirection :type Vector :default "0, 0, 0") (PushForce :type Float%20%28single-precision%29))
  (Class|PhysicalInteract|ReleaseObject))

(event EventTick
  (params (DeltaSeconds :type Float%20%28single-precision%29))
  (bind _initialrestlocation (Variables|Default|GetInitialRestLocation))
  (bind (_x _y _z) (Math|Vector|BreakVector _initialrestlocation))
  (|CallParentFunction DeltaSeconds)
  (Transformation|SetRelativeLocation (Variables|Default|GetDrawerMesh) (Math|Vector|MakeVector _x (Math|Interpolation|FInterpTo (.Y (Math|Vector|BreakVector (Variables|/Script/Engine.SceneComponent|GetRelativeLocation (Variables|Default|GetDrawerMesh)))) (+ (.Y (Math|Vector|BreakVector (Variables|Default|GetInitialRestLocation))) (Variables|Default|GetDrawerSlideDistance)) DeltaSeconds 8.0) _z) false false))

(event EventGrabObject
  (params (Grabber :type Actor%20Object%20Reference))
  ;[0.15 0.15 0.15 0.5] grab door
  (Variables|Default|SetbIsLatched false)
  (|CallParentFunction Grabber)
  (Development|PrintString "klik"))

(event EventMoveObject
  (params (AxisDelta :type Float%20%28single-precision%29))
  ;[0.15 0.15 0.15 0.5] move door
  (Variables|Default|SetDrawerSlideDistance (Math|Float|Clamp(Float) (+ (* (* (* (Variables|Default|GetBaseInteractionPower) AxisDelta) (Class|BaseInteractable|CalculateMovementResistance (Variables|Default|GetDrawerMesh))) 0.05) (Variables|Default|GetDrawerSlideDistance)) 0.0 (Variables|Default|GetMaxOpenDist))))

(event EventReleaseObject
  ;[0.15 0.15 0.15 0.5] release door
  (Variables|Default|SetbIsLatched false)
  (if (and (<= (Variables|Default|GetDrawerSlideDistance) 1.0) (Variables|Default|GetbIsHeld))
    (Variables|Default|SetbIsLatched true))
  (|CallParentFunction))

(fn ConstructionScript
  (|CallParentFunction)
  (Class|PhysicsConstraintComponent|SetLinearXLimit (Variables|Default|GetPhysicsConstraint) "LCM_Limited" (Variables|Default|GetDrawerSlideDistance)))